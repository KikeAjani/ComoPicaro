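; An explosive grenade projectile that launches with a set physics velocity and damages enemies where it hits.
; Each hit on another actor spawns explosion particles and sound, then sphere-overlaps around the impact and calls Damage on every Enemy found.
; Tick accumulates time since spawn, and the actor destroys itself only on a hit after a few seconds, so earlier bounces can explode repeatedly.
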(event OnComponentHit(Sphere)
  (params (HitComponent :type Primitive%20Component%20Object%20Reference) (OtherActor :type Actor%20Object%20Reference) (OtherComp :type Primitive%20Component%20Object%20Reference) (NormalImpulse :type Vector :default "0, 0, 0") (Hit :type Hit%20Result%20Structure%20%28by%20ref%29)))

(event Collision|EventHit
  (params (MyComp :type Primitive%20Component%20Object%20Reference) (Other :type Actor%20Object%20Reference) (OtherComp :type Primitive%20Component%20Object%20Reference) (bSelfMoved :type Boolean) (HitLocation :type Vector :default "0, 0, 0") (HitNormal :type Vector :default "0, 0, 0") (NormalImpulse :type Vector :default "0, 0, 0") (Hit :type Hit%20Result%20Structure%20%28by%20ref%29))
  (if (!= Other self)
    (bind _returnvalue (Effects|SpawnEmitteratLocation "/Game/StarterContent/Particles/P_Explosion.P_Explosion" HitLocation "0, 0, 0" "2.000000,2.000000,2.000000"))
    (Audio|SpawnSoundAttached "/Game/StarterContent/Audio/Explosion01.Explosion01" _returnvalue "None" "0, 0, 0" "0, 0, 0" "KeepRelativeOffset" false 0.1 1.0 0.0 0 0)
    (bind _outactors (Collision|SphereOverlapActors HitLocation 2e+02 (Utilities|Array|MakeArray "ObjectTypeQuery10") 0))
    (for _array_element _outactors
      (bind _asenemy (Utilities|Casting|CastToEnemy _array_element))
      (Class|Enemy|Damage _asenemy 500))
    (if (>= (Variables|Default|GetUltimateSeconds) 3.0)
      (Actor|DestroyActor))))

(event Collision|EventActorBeginOverlap
  (params (OtherActor :type Actor%20Object%20Reference)))

(event EventTick
  (params (DeltaSeconds :type Float%20%28single-precision%29))
  (Variables|Default|SetUltimateSeconds (+ DeltaSeconds (Variables|Default|GetUltimateSeconds))))

(event EventBeginPlay
  (Physics|SetPhysicsLinearVelocity (Variables|Default|GetGrenade) (Variables|Default|GetGrenadeVelocity) false "None")
  (Variables|Default|SetUltimateSeconds 0.0))

(fn ConstructionScript)