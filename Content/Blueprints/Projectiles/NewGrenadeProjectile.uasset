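; NewGrenadeProjectile is a timed grenade projectile Blueprint that explodes after a fixed fuse.
; On BeginPlay it applies its velocity as an impulse to the sphere and fires the radial force immediately, before the fuse delay.
; After the delay it spawns explosion particles with attached sound and destroys itself.
; Any actor overlap destroys it early, then calls an add-particle node with no template shown.
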(event EventBeginPlay
  (Physics|AddImpulseatLocation (Variables|Default|GetSphere) (Transformation|GetVelocity) (Transformation|GetActorLocation) "None")
  (Class|RadialForceComponent|FireImpulse (Variables|Default|GetRadialForce))
  (Utilities|FlowControl|Delay 3.0)
  (bind _returnvalue (Effects|SpawnEmitteratLocation "/Game/StarterContent/Particles/P_Explosion.P_Explosion" (Transformation|GetActorLocation)))
  (Audio|SpawnSoundAttached "/Game/StarterContent/Audio/Explosion01.Explosion01" _returnvalue "None" "0, 0, 0" "0, 0, 0" "KeepRelativeOffset" false 1.0 1.0 0.0 0 0)
  (Actor|DestroyActor))

(event Collision|EventActorBeginOverlap
  (params (OtherActor :type Actor%20Object%20Reference))
  (Actor|DestroyActor)
  (AddComponent|AddParticleSystemComponent false))

(event EventTick
  (params (DeltaSeconds :type Float%20%28single-precision%29)))

(fn ConstructionScript)