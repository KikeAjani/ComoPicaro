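; Level-exit portal that advances the run when the MainCharacter overlaps it.
; On overlap it saves player info through ComoPicaroGameInstance_BP, then raises the level difficulty and level number stored there.
; It opens the boss level when the level counter reaches six, otherwise it reloads the base persistent room map for the next level.
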(event Collision|EventActorBeginOverlap
  (params (OtherActor :type Actor%20Object%20Reference))
  (Utilities|Casting|CastToMainCharacter OtherActor)
  (bind _ascomo_picaro_game_instance_bp (Utilities|Casting|CastToComoPicaroGameInstance_BP (Game|GetGameInstance)))
  (Default|SavePlayerInfo _ascomo_picaro_game_instance_bp)
  (Variables|/Script/ComoPicaro.ComoPicaroGameInstance|SetLevelDificulty _ascomo_picaro_game_instance_bp (+ (Variables|/Script/ComoPicaro.ComoPicaroGameInstance|GetLevelDificulty _ascomo_picaro_game_instance_bp) 5))
  (bind _output_get (Variables|/Script/ComoPicaro.ComoPicaroGameInstance|SetNumLevel _ascomo_picaro_game_instance_bp (+ (Variables|/Script/ComoPicaro.ComoPicaroGameInstance|GetNumLevel _ascomo_picaro_game_instance_bp) 1)))
  (if (== _output_get 6)
    (Game|OpenLevel(byName) "BossLevel1")
    (else
      (Game|OpenLevel(byName) "BasePersistentRoomMap"))))

(fn ConstructionScript)