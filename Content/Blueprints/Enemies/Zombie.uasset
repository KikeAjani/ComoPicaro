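; Zombie enemy Blueprint that displays a health bar and moans periodically.
; BeginPlay plays one of two moan sounds at random at the actor's location.
; Tick pushes current and initial health to the EnemyHPBar widget, then accumulates delta time to replay the random moan roughly every five seconds.
; The moan timer runs only when the widget cast succeeds.
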(event EventBeginPlay
  (bind _returnvalue (Transformation|GetActorLocation))
  (if (== (Math|Random|RandomInteger 2) 0)
    (Audio|PlaySoundatLocation "/Game/Resources/Enemies/Zombie/SFX/Zombie_Moan.Zombie_Moan" _returnvalue "0, 0, 0" 1.0 1.0 0.0 0 0 0)
    (else
      (Audio|PlaySoundatLocation "/Game/Resources/Enemies/Zombie/SFX/Mummy_Zombie.Mummy_Zombie" _returnvalue "0, 0, 0" 1.0 1.0 0.0 0 0 0))))

(event EventTick
  (params (DeltaSeconds :type Float%20%28single-precision%29))
  (bind _returnvalue (Transformation|GetActorLocation))
  (bind _asenemy_hpbar (Utilities|Casting|CastToEnemyHPBar (UserInterface|GetUserWidgetObject (Variables|Default|GetEnemyHPBar))))
  (Default|UpdateHealth _asenemy_hpbar (Math|Conversions|ToFloat(Integer) (Variables|Default|GetHealth)) (Math|Conversions|ToFloat(Integer) (Variables|Default|GetInitialHealth)))
  (bind _output_get (Variables|Default|SetTimeSinceLastMoan (+ (Variables|Default|GetTimeSinceLastMoan) (Utilities|Time|GetWorldDeltaSeconds))))
  (if (> _output_get 5.0)
    (Variables|Default|SetTimeSinceLastMoan 0.0)
    (if (== (Math|Random|RandomInteger 2) 0)
      (Audio|PlaySoundatLocation "/Game/Resources/Enemies/Zombie/SFX/Zombie_Moan.Zombie_Moan" _returnvalue "0, 0, 0" 1.0 1.0 0.0 0 0 0)
      (else
        (Audio|PlaySoundatLocation "/Game/Resources/Enemies/Zombie/SFX/Mummy_Zombie.Mummy_Zombie" _returnvalue "0, 0, 0" 1.0 1.0 0.0 0 0 0)))))

(fn ConstructionScript)