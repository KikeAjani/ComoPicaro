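; Warrok is a boss enemy Blueprint that displays its health on screen through a BossHUD widget.
; BeginPlay creates the widget, adds it to the viewport and feeds it current and initial health.
; Tick repeats that whole sequence, so a new widget is added every frame rather than the existing one being updated.
; A DeadParticles function adds a particle component but is not called here, and a Dying check is left unconnected.
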(event EventBeginPlay
  (bind _returnvalue (UserInterface|CreateWidget "/Game/Blueprints/Widgets/BossHUD.BossHUD_C"))
  (bind _output_get (Variables|Default|SetEnemyHPBoss _returnvalue))
  (UserInterface|Viewport|AddtoViewport _output_get 0)
  (Default|UpdateHealth (Variables|Default|GetEnemyHPBoss) (Math|Conversions|ToFloat(Integer) (Variables|Default|GetHealth)) (Math|Conversions|ToFloat(Integer) (Variables|Default|GetInitialHealth))))

(event Collision|EventActorBeginOverlap
  (params (OtherActor :type Actor%20Object%20Reference)))

(event EventTick
  (params (DeltaSeconds :type Float%20%28single-precision%29))
  (bind _returnvalue (UserInterface|CreateWidget "/Game/Blueprints/Widgets/BossHUD.BossHUD_C"))
  (bind _output_get (Variables|Default|SetEnemyHPBoss _returnvalue))
  (UserInterface|Viewport|AddtoViewport _output_get 0)
  (Default|UpdateHealth (Variables|Default|GetEnemyHPBoss) (Math|Conversions|ToFloat(Integer) (Variables|Default|GetHealth)) (Math|Conversions|ToFloat(Integer) (Variables|Default|GetInitialHealth))))

(fn ConstructionScript)

(fn DeadParticles
  (AddComponent|AddParticleSystemComponent false))