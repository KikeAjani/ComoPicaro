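; Mutant is an enemy Blueprint that keeps a floating health bar widget up to date and turned toward the player.
; Each Tick casts the widget component's object to EnemyHPBar and passes it current and initial health as floats.
; It then rotates the component with a look-at toward a point slightly above the player character's location.
; The graphs shown contain no other behavior.
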(event EventBeginPlay)

(event Collision|EventActorBeginOverlap
  (params (OtherActor :type Actor%20Object%20Reference)))

(event EventTick
  (params (DeltaSeconds :type Float%20%28single-precision%29))
  (bind _enemyhpbar (Variables|Default|GetEnemyHPBar))
  (bind _asenemy_hpbar (Utilities|Casting|CastToEnemyHPBar (UserInterface|GetUserWidgetObject (Variables|Default|GetEnemyHPBar))))
  (Default|UpdateHealth _asenemy_hpbar (Math|Conversions|ToFloat(Integer) (Variables|Default|GetHealth)) (Math|Conversions|ToFloat(Integer) (Variables|Default|GetInitialHealth)))
  (Transformation|SetWorldRotation _enemyhpbar (Math|Rotator|FindLookatRotation (Transformation|GetWorldLocation _enemyhpbar) (+ (Transformation|GetActorLocation (Game|GetPlayerCharacter 0)) "0, 0,90.000000")) false false))

(fn ConstructionScript)