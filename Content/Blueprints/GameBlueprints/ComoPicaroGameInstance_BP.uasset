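; Game instance for ComoPicaro that carries the main character's progression from one level to the next.
; Save copies health, simple attack speed and extra damage, ultimate points and the count of tagged fire components from the player character.
; Load writes those stats back on every level except the first, then has the game mode re-add arrow projectiles for each saved fire component beyond the first.
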(fn LoadPlayerInfo
  (if (not (== (Variables|Default|GetNumLevel) 1))
    (bind _asmain_character (Utilities|Casting|CastToMainCharacter (Game|GetPlayerCharacter 0)))
    (Variables|/Script/ComoPicaro.MainCharacter|SetActualHealth _asmain_character (Variables|Default|GetActualHealth))
    (Variables|/Script/ComoPicaro.MainCharacter|SetHealth _asmain_character (Variables|Default|GetHealth))
    (Variables|/Script/ComoPicaro.MainCharacter|SetSimpleAttackSpeed _asmain_character (Variables|Default|GetSimpleAttackSpeed))
    (Variables|/Script/ComoPicaro.MainCharacter|SetPointsToUltimate _asmain_character (Variables|Default|GetPointsToUltimate))
    (Variables|/Script/ComoPicaro.MainCharacter|SetExtraDamageSimpleAttack _asmain_character (Variables|Default|GetExtraDamageSimpleAttack))
    (bind _ascomo_picaro_game_mode_bp (Utilities|Casting|CastToComoPicaroGameMode_BP (Game|GetGameMode)))
    (for _index (range 1 (- (Variables|Default|GetNumOfFireComponents) 1))
      (Default|AddArrowProjectile _ascomo_picaro_game_mode_bp _asmain_character))))

(fn SavePlayerInfo
  (bind _asmain_character (Utilities|Casting|CastToMainCharacter (Game|GetPlayerCharacter 0)))
  (Variables|Default|SetActualHealth (Variables|/Script/ComoPicaro.MainCharacter|GetActualHealth _asmain_character))
  (Variables|Default|SetHealth (Variables|/Script/ComoPicaro.MainCharacter|GetHealth _asmain_character))
  (Variables|Default|SetSimpleAttackSpeed (Variables|/Script/ComoPicaro.MainCharacter|GetSimpleAttackSpeed _asmain_character))
  (Variables|Default|SetPointsToUltimate (Variables|/Script/ComoPicaro.MainCharacter|GetPointsToUltimate _asmain_character))
  (Variables|Default|SetExtraDamageSimpleAttack (Variables|/Script/ComoPicaro.MainCharacter|GetExtraDamageSimpleAttack _asmain_character))
  (Variables|Default|SetNumOfFireComponents (Utilities|Array|Length (Actor|GetComponentsbyTag _asmain_character "/Script/ComoPicaro.FireComponent" "FireComponent"))))