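; Game mode Blueprint that provides a function to add another arrow projectile to the main character.
; AddArrowProjectile adds a fire component that copies the projectile class of the character's main fire component.
; It then re-spreads every component tagged FireComponent along the Y spawn offset, using different spacing for even and odd counts and taking X and Z from the main component.
; The event graph and construction script are empty.
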(event EventBeginPlay)

(event EventTick
  (params (DeltaSeconds :type Float%20%28single-precision%29)))

(fn ConstructionScript)

(fn AddArrowProjectile
  (params (MainCharacter :type Main%20Character%20Object%20Reference))
  (bind _returnvalue (Actor|GetComponentsbyTag MainCharacter "/Script/ComoPicaro.FireComponent" "FireComponent"))
  (bind _mfirecomponent (Variables|/Script/ComoPicaro.MainCharacter|GetMFireComponent MainCharacter))
  (bind _returnvalue_2 (Utilities|Array|Length _returnvalue))
  (bind _returnvalue_3 (/ _returnvalue_2 2))
  (bind _returnvalue_4 (AddComponent|AddFireComponent MainCharacter))
  (Variables|/Script/ComoPicaro.FireComponent|SetProjectileClass _returnvalue_4 (Variables|/Script/ComoPicaro.FireComponent|GetProjectileClass _mfirecomponent))
  (if (== (Math|Integer|%(Integer) _returnvalue_2 2) 0)
    (for (_array_element _array_index) _returnvalue
      (Variables|/Script/ComoPicaro.FireComponent|SetSpawnOffset _array_element (Math|Vector|MakeVector (.x (Variables|/Script/ComoPicaro.FireComponent|GetSpawnOffset _mfirecomponent)) (+ (- 3.0 (Math|Conversions|ToFloat(Integer) (* (- _returnvalue_3 1) 20))) (Math|Conversions|ToFloat(Integer) (* _array_index 20))) (.z (Variables|/Script/ComoPicaro.FireComponent|GetSpawnOffset _mfirecomponent)))))
    (else
      (for (_array_element_2 _array_index_2) _returnvalue
        (Variables|/Script/ComoPicaro.FireComponent|SetSpawnOffset _array_element_2 (Math|Vector|MakeVector (.x (Variables|/Script/ComoPicaro.FireComponent|GetSpawnOffset _mfirecomponent)) (Math|Conversions|ToFloat(Integer) (+ (* _array_index_2 15) (- 13 (* _returnvalue_3 15)))) (.z (Variables|/Script/ComoPicaro.FireComponent|GetSpawnOffset _mfirecomponent))))))))