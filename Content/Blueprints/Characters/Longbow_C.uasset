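; Player Blueprint for the Longbow archer, handling attacks, HUD, footsteps and pause menu.
; Tick repeats the simple attack while left-click is held, sets the running animation, updates health and plays speed-timed footsteps via Delay.
; The ultimate lobs a grenade at the cursor using a suggested toss velocity.
; AddArrowProjectile adds fire components and spreads their spawn offsets laterally, with separate even and odd layouts.
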(event Collision|EventActorBeginOverlap
  (params (OtherActor :type Actor%20Object%20Reference)))

(event EventTick
  (params (DeltaSeconds :type Float%20%28single-precision%29))
  (bind _charactermovement (Variables|Character|GetCharacterMovement))
  (bind _mesh (Variables|Character|GetMesh))
  (bind _returnvalue (Components|SkeletalMesh|GetAnimInstance _mesh))
  (bind _velocity (Variables|/Script/Engine.MovementComponent|GetVelocity _charactermovement))
  (bind _returnvalue_2 (Math|Vector|VectorLength _velocity))
  (if (Variables|Default|GetIsLeftClickPressed)
    (Class|MainCharacter|OnSimpleAttack))
  (if (or (!= (Input|AxisValues|GetMoveRight) 0.0) (!= (Input|AxisValues|GetMoveForward) 0.0))
    (bind _aslongbow_animation_instance_bp (Utilities|Casting|CastToLongbowAnimationInstance_BP _returnvalue))
    (Variables|/Script/ComoPicaro.LongbowAnimationInstance|SetIsRunning _aslongbow_animation_instance_bp true)
    (else
      (bind _aslongbow_animation_instance_bp_2 (Utilities|Casting|CastToLongbowAnimationInstance_BP _returnvalue))
      (Variables|/Script/ComoPicaro.LongbowAnimationInstance|SetIsRunning _aslongbow_animation_instance_bp_2 false)))
  (Default|UpdateHealth (Variables|Default|GetHUDRef) (Math|Conversions|ToFloat(Integer) (Variables|Default|GetActualHealth)) (Math|Conversions|ToFloat(Integer) (Variables|Default|GetHealth)))
  ;[1 1 1] Steps Soound
  (if (not (< _returnvalue_2 3e+01))
    (Utilities|FlowControl|Delay (Math|Float|MapRangeClamped _returnvalue_2 0.0 3.6e+02 1.0 0.4))
    (if (not (< _returnvalue_2 3e+01))
      (Audio|PlaySoundatLocation "/Game/TwinStick/Audio/Steps/StepGravel.StepGravel" (Transformation|GetActorLocation) "0, 0, 0" 1.0 1.0 0.0 0 0 0))))

(event EventBeginPlay
  (bind _returnvalue (UserInterface|CreateWidget "/Game/Blueprints/Widgets/HUD.HUD_C"))
  (bind _output_get (Variables|Default|SetHUDRef _returnvalue))
  (UserInterface|Viewport|AddtoViewport _output_get 0)
  (Default|UpdateHealth (Variables|Default|GetHUDRef) (Math|Conversions|ToFloat(Integer) (Variables|Default|GetActualHealth)) (Math|Conversions|ToFloat(Integer) (Variables|Default|GetHealth))))

(event EventMUltimate
  (bind _billboard (Variables|Default|GetBillboard))
  (bind _aslongbow_animation_instance (Utilities|Casting|CastToLongbowAnimationInstance (Components|SkeletalMesh|GetAnimInstance (Variables|Character|GetMesh))))
  (Variables|/Script/ComoPicaro.LongbowAnimationInstance|SetIsUltimating _aslongbow_animation_instance true)
  (Utilities|FlowControl|Delay 0.2)
  (bind _tossvelocity (Class|GameplayStatics|BlueprintSuggestProjectileVelocity (Transformation|GetWorldLocation (Variables|Default|GetBillboard)) (.Location (Collision|BreakHitResult (.HitResult (Game|Player|GetHitResultUnderCursorbyChannel (Game|GetPlayerController 0) "TraceTypeQuery1" true)))) 1.5e+03 0.0 "DoNotTrace" 0.0 false false))
  (Game|SpawnActorfromClass "/Game/Blueprints/Projectiles/GrenadeProjectile.GrenadeProjectile_C" (Math|Transform|MakeTransform (Transformation|GetWorldLocation _billboard) "0, 0, 0" "0.200000,0.200000,0.200000") "AdjustIfPossibleButAlwaysSpawn" 0 _tossvelocity 0)
  (Transformation|SetWorldRotation _billboard (Transformation|GetWorldRotation (Variables|Character|GetMesh)) false false))

(event Input|ActionEvents|InputActionSimpleAttack
  (params (Key :type Key%20Structure :default "None")))

(event Input|KeyboardEvents|P
  (params (Key :type Key%20Structure :default "None"))
  (:Pressed
    (CallFunction|PauseGame)))

(fn ConstructionScript)

(fn AddArrowProjectile
  (bind _returnvalue (Actor|GetComponentsbyTag "/Script/ComoPicaro.FireComponent" "FireComponent"))
  (bind _mfirecomponent (Variables|Default|GetMFireComponent))
  (bind _returnvalue_2 (Utilities|Array|Length _returnvalue))
  (bind _returnvalue_3 (/ _returnvalue_2 2))
  (bind _returnvalue_4 (AddComponent|AddFireComponent self))
  (Variables|/Script/ComoPicaro.FireComponent|SetProjectileClass _returnvalue_4 (Variables|/Script/ComoPicaro.FireComponent|GetProjectileClass _mfirecomponent))
  (if (== (Math|Integer|%(Integer) _returnvalue_2 2) 0)
    (for (_array_element _array_index) _returnvalue
      (Variables|/Script/ComoPicaro.FireComponent|SetSpawnOffset _array_element (Math|Vector|MakeVector (.x (Variables|/Script/ComoPicaro.FireComponent|GetSpawnOffset _mfirecomponent)) (+ (- 3.0 (Math|Conversions|ToFloat(Integer) (* (- _returnvalue_3 1) 20))) (Math|Conversions|ToFloat(Integer) (* _array_index 20))) (.z (Variables|/Script/ComoPicaro.FireComponent|GetSpawnOffset _mfirecomponent)))))
    (else
      (for (_array_element_2 _array_index_2) _returnvalue
        (Variables|/Script/ComoPicaro.FireComponent|SetSpawnOffset _array_element_2 (Math|Vector|MakeVector (.x (Variables|/Script/ComoPicaro.FireComponent|GetSpawnOffset _mfirecomponent)) (Math|Conversions|ToFloat(Integer) (+ (* _array_index_2 15) (- 13 (* _returnvalue_3 15)))) (.z (Variables|/Script/ComoPicaro.FireComponent|GetSpawnOffset _mfirecomponent))))))))

(fn PauseGame
  (Game|SetGamePaused true)
  (Utilities|IsValid (Variables|Default|GetPauseMenu)
    (:Is%20Valid
      _)
    (:Is%20Not%20Valid
      (bind _returnvalue (UserInterface|CreateWidget "/Game/MainMenu/PauseMenu.PauseMenu_C" (Game|GetPlayerController 0)))
      (Variables|Default|SetPauseMenu _returnvalue)))
  (UserInterface|Viewport|AddtoViewport (Variables|Default|GetPauseMenu) 0)
  (Input|SetInputModeUIOnly (Game|GetPlayerController 0) (Variables|Default|GetPauseMenu) "DoNotLock"))

(fn UnpauseGame
  (Game|SetGamePaused false)
  (Viewport|RemoveAllWidgets)
  (Input|SetInputModeGameandUI (Game|GetPlayerController 0) 0 "DoNotLock" false))