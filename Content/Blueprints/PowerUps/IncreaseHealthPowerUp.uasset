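; IncreaseHealthPowerUp is a pickup that boosts the main character's health when touched.
; On overlap with a MainCharacter, it calls Actuate, registers itself through AddHability, then destroys its own actor.
; Actuate adds a fixed bonus to both the character's Health and ActualHealth.
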(event EventBeginPlay)

(event EventTick
  (params (DeltaSeconds :type Float%20%28single-precision%29)))

(event EventActuate
  (params (MainCharacter :type Main%20Character%20Object%20Reference))
  (Variables|/Script/ComoPicaro.MainCharacter|SetHealth MainCharacter (+ (Variables|/Script/ComoPicaro.MainCharacter|GetHealth MainCharacter) 10))
  (Variables|/Script/ComoPicaro.MainCharacter|SetActualHealth MainCharacter (+ (Variables|/Script/ComoPicaro.MainCharacter|GetActualHealth MainCharacter) 10)))

(event Collision|EventActorBeginOverlap
  (params (OtherActor :type Actor%20Object%20Reference))
  (bind _asmain_character (Utilities|Casting|CastToMainCharacter OtherActor))
  (Default|Actuate self _asmain_character)
  (Class|MainCharacter|AddHability _asmain_character self)
  (Actor|DestroyActor))

(fn ConstructionScript)