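; AddProjectilePowerUp is a pickup that grants the main character an extra arrow projectile when they overlap it.
; On overlap, Actuate asks ComoPicaroGameMode_BP to add the arrow projectile, then calls AddHability on the character and destroys the pickup.
; An unconnected older branch that added a fire component and spread spawn offsets by even or odd count remains but never runs.
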(event EventBeginPlay)

(event EventActuate
  (params (MainCharacter :type Main%20Character%20Object%20Reference))
  (bind _ascomo_picaro_game_mode_bp (Utilities|Casting|CastToComoPicaroGameMode_BP (Game|GetGameMode)))
  (Default|AddArrowProjectile _ascomo_picaro_game_mode_bp MainCharacter)
  (Class|MainCharacter|AddHability MainCharacter)
  (Actor|DestroyActor))

(event EventTick
  (params (DeltaSeconds :type Float%20%28single-precision%29)))

(event Collision|EventActorBeginOverlap
  (params (OtherActor :type Actor%20Object%20Reference))
  (bind _asmain_character (Utilities|Casting|CastToMainCharacter OtherActor))
  (CallFunction|Actuate _asmain_character))

(fn ConstructionScript)